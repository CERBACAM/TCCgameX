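; Blood decal Blueprint that randomizes its decal material when it spawns.
; On BeginPlay it rolls a random integer into Numero, and a chain of threshold checks sets the matching blood material instance on the Decal component.
; The last check follows the previous one's true branch, so a roll of 7 sets Inst7 and immediately replaces it with Inst8.
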(event `self.ReceiveBeginPlay`
  (set `self.numero` (`KismetMathLibrary.RandomInteger` 8))
  (if (<= (`self.numero`) 0)
    (`DecalComponent.SetDecalMaterial` (`self.Decal`) "/Game/zTUDO/materiais/blood/Blood_Decal_M_Inst.Blood_Decal_M_Inst")
    (elif (<= (`self.numero`) 1)
      (`DecalComponent.SetDecalMaterial` (`self.Decal`) "/Game/zTUDO/materiais/blood/Blood_Decal_M_Inst_Inst1.Blood_Decal_M_Inst_Inst1")
      (elif (<= (`self.numero`) 2)
        (`DecalComponent.SetDecalMaterial` (`self.Decal`) "/Game/zTUDO/materiais/blood/Blood_Decal_M_Inst_Inst2.Blood_Decal_M_Inst_Inst2")
        (elif (<= (`self.numero`) 3)
          (`DecalComponent.SetDecalMaterial` (`self.Decal`) "/Game/zTUDO/materiais/blood/Blood_Decal_M_Inst_Inst3.Blood_Decal_M_Inst_Inst3")
          (elif (<= (`self.numero`) 4)
            (`DecalComponent.SetDecalMaterial` (`self.Decal`) "/Game/zTUDO/materiais/blood/Blood_Decal_M_Inst_Inst4.Blood_Decal_M_Inst_Inst4")
            (elif (<= (`self.numero`) 5)
              (`DecalComponent.SetDecalMaterial` (`self.Decal`) "/Game/zTUDO/materiais/blood/Blood_Decal_M_Inst_Inst5.Blood_Decal_M_Inst_Inst5")
              (elif (<= (`self.numero`) 6)
                (`DecalComponent.SetDecalMaterial` (`self.Decal`) "/Game/zTUDO/materiais/blood/Blood_Decal_M_Inst_Inst6.Blood_Decal_M_Inst_Inst6")
                (elif (<= (`self.numero`) 7)
                  (`DecalComponent.SetDecalMaterial` (`self.Decal`) "/Game/zTUDO/materiais/blood/Blood_Decal_M_Inst_Inst7.Blood_Decal_M_Inst_Inst7")
                  (if (<= (`self.numero`) 8)
                    (`DecalComponent.SetDecalMaterial` (`self.Decal`) "/Game/zTUDO/materiais/blood/Blood_Decal_M_Inst_Inst8.Blood_Decal_M_Inst_Inst8")))))))))))

(fn `UserConstructionScript`)